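; Physics-driven satellite actor that moves and rotates with 24 particle thrusters, grouped as three axes on each of eight vertices.
; ThrustByVector fires thrusters by dot product with the requested vector, applying opposing impulses at their locations.
; Rotate derives per-vertex tangential thrust from a cross-product axis.
; Tick expires thruster effects by timer, adds constant upward lift, and calls Move through Hover whenever below the target height.
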(event EventTick
  (params (DeltaSeconds :type Float%20%28single-precision%29))
  (CallFunction|Update DeltaSeconds))

(fn ConstructionScript
  (bind _thrustofftimer (Variables|Default|GetThrustOffTimer))
  (Utilities|Array|Resize (Variables|Default|GetThrustes) 24)
  (Utilities|Array|SetArrayElem (Variables|Default|GetThrustes) 0 (Variables|Default|GetThrush1_X))
  (Utilities|Array|SetArrayElem (Variables|Default|GetThrustes) 1 (Variables|Default|GetThrush1_Y))
  (Utilities|Array|SetArrayElem (Variables|Default|GetThrustes) 2 (Variables|Default|GetThrush1_Z))
  (Utilities|Array|SetArrayElem (Variables|Default|GetThrustes) 3 (Variables|Default|GetThrust2_NX))
  (Utilities|Array|SetArrayElem (Variables|Default|GetThrustes) 4 (Variables|Default|GetThrust2_Y))
  (Utilities|Array|SetArrayElem (Variables|Default|GetThrustes) 5 (Variables|Default|GetThrust2_Z))
  (Utilities|Array|SetArrayElem (Variables|Default|GetThrustes) 6 (Variables|Default|GetThrust3_NX))
  (Utilities|Array|SetArrayElem (Variables|Default|GetThrustes) 7 (Variables|Default|GetThrust3_NY))
  (Utilities|Array|SetArrayElem (Variables|Default|GetThrustes) 8 (Variables|Default|GetThrust3_Z))
  (Utilities|Array|SetArrayElem (Variables|Default|GetThrustes) 9 (Variables|Default|GetThrust4_X))
  (Utilities|Array|SetArrayElem (Variables|Default|GetThrustes) 10 (Variables|Default|GetThrust4_NY))
  (Utilities|Array|SetArrayElem (Variables|Default|GetThrustes) 11 (Variables|Default|GetThrust4_Z))
  (Utilities|Array|SetArrayElem (Variables|Default|GetThrustes) 12 (Variables|Default|GetThrust5_X))
  (Utilities|Array|SetArrayElem (Variables|Default|GetThrustes) 13 (Variables|Default|GetThrust5_Y))
  (Utilities|Array|SetArrayElem (Variables|Default|GetThrustes) 14 (Variables|Default|GetThrust5_NZ))
  (Utilities|Array|SetArrayElem (Variables|Default|GetThrustes) 15 (Variables|Default|GetThrust6_NX))
  (Utilities|Array|SetArrayElem (Variables|Default|GetThrustes) 16 (Variables|Default|GetThrust6_Y))
  (Utilities|Array|SetArrayElem (Variables|Default|GetThrustes) 17 (Variables|Default|GetThrust6_NZ))
  (Utilities|Array|SetArrayElem (Variables|Default|GetThrustes) 18 (Variables|Default|GetThrust7_NX))
  (Utilities|Array|SetArrayElem (Variables|Default|GetThrustes) 19 (Variables|Default|GetThrust7_NY))
  (Utilities|Array|SetArrayElem (Variables|Default|GetThrustes) 20 (Variables|Default|GetThrust7_NZ))
  (Utilities|Array|SetArrayElem (Variables|Default|GetThrustes) 21 (Variables|Default|GetThrust8_X))
  (Utilities|Array|SetArrayElem (Variables|Default|GetThrustes) 22 (Variables|Default|GetThrust8_NY))
  (Utilities|Array|SetArrayElem (Variables|Default|GetThrustes) 23 (Variables|Default|GetThrust8_NZ))
  ;[1 1 1] Init Thrust Vertex Direction
  (CallFunction|InitThrustVertexPoint)
  ;[1 1 1] Init Vertex Rotate Direction
  (CallFunction|InitVertexRotateDirection)
  ;[1 1 1] Init Tangent Space Transform
  (CallFunction|InitTangentSpaceTransform)
  ;[1 1 1] Init Thrust Off Timer
  (Utilities|Array|Resize _thrustofftimer 24)
  (for (_ _array_index) _thrustofftimer
    (Utilities|Array|SetArrayElem _thrustofftimer _array_index -1.0)))

(fn Thrust
  (params (ThrustIndex :type Integer) (Power :type Float%20%28single-precision%29))
  (bind _thrustes (Variables|Default|GetThrustes))
  (bind _item (Utilities|Array|Get(acopy) _thrustes ThrustIndex))
  (LocalVariables|SetThrustIdx ThrustIndex)
  (if (< ThrustIndex 24)
    (if (Components|Activation|IsActive _item)
      _
      (else
        (Components|Activation|SetActive _item true true)))
    (Effects|Components|ParticleSystem|SetEmitterEnable _item "Particle Emitter" true)
    (Physics|AddImpulseatLocation (Variables|Default|GetStaticMesh1) (Math|Vector|NegateVector (* (Math|Vector|GetForwardVector (Transformation|GetWorldRotation _item)) Power)) (Transformation|GetWorldLocation _item) "None")
    (Utilities|Array|SetArrayElem (Variables|Default|GetThrustOffTimer) (LocalVariables|GetThrustIdx) 1.0)))

(fn ThrustOff
  (params (ThrustIndex :type Integer))
  (if (< ThrustIndex 24)
    (Effects|Components|ParticleSystem|SetEmitterEnable (Utilities|Array|Get(acopy) (Variables|Default|GetThrustes) ThrustIndex) "Particle Emitter" false)))

(fn Rotate
  (params (Direction :type Vector))
  ;[1 1 1] Calculate Rotate Axis
  (LocalVariables|SetRotateAxis (Math|Vector|Normalize (Math|Vector|CrossProduct (Math|Vector|GetForwardVector (Transformation|GetWorldRotation (Variables|Default|GetStaticMesh1))) Direction)))
  (for (_ _array_index) (Variables|Default|GetTangentSpaceTransforms)
    (LocalVariables|SetIndex _array_index)
    (Transformation|SetWorldRotation (Utilities|Array|Get(acopy) (Variables|Default|GetVertexRotateDirection) (LocalVariables|GetIndex)) (Math|Rotator|MakeRotfromZY (Math|Vector|RotateVector (Utilities|Array|Get(acopy) (Variables|Default|GetVertexDirection) _array_index) (Transformation|GetWorldRotation (Variables|Default|GetStaticMesh1))) (LocalVariables|GetRotateAxis)) false)
    (CallFunction|ThrustbyVector (LocalVariables|GetIndex) (Math|Vector|NegateVector (Math|Vector|GetForwardVector (Math|Rotator|MakeRotfromZY (Math|Vector|RotateVector (Utilities|Array|Get(acopy) (Variables|Default|GetVertexDirection) _array_index) (Transformation|GetWorldRotation (Variables|Default|GetStaticMesh1))) (LocalVariables|GetRotateAxis)))) 1e+03)))

(fn InitThrustVertexPoint
  (bind _thrustes (Variables|Default|GetThrustes))
  (bind _returnvalue (Utilities|Array|Length _thrustes))
  (Utilities|Array|Resize (Variables|Default|GetVertexDirection) (/ _returnvalue 3))
  (LocalVariables|Setindex 0)
  (while (< (LocalVariables|Getindex) _returnvalue)
    ;[1 1 1] Calculate Thrust Vector
    (bind _returnvalue_2 (Transformation|GetRelativeTransform (Utilities|Array|Get(acopy) (Variables|Default|GetThrustes) (LocalVariables|Getindex))))
    (bind _returnvalue_3 (Transformation|GetRelativeTransform (Utilities|Array|Get(acopy) (Variables|Default|GetThrustes) (+ (LocalVariables|Getindex) 1))))
    (bind _returnvalue_4 (Transformation|GetRelativeTransform (Utilities|Array|Get(acopy) (Variables|Default|GetThrustes) (+ (LocalVariables|Getindex) 2))))
    (Utilities|Array|SetArrayElem (Variables|Default|GetVertexDirection) (/ (LocalVariables|Getindex) 3) (Math|Vector|Normalize (+ (.Location (Math|Transform|BreakTransform _returnvalue_2)) (.Location (Math|Transform|BreakTransform _returnvalue_3)) (.Location (Math|Transform|BreakTransform _returnvalue_4)))))
    (LocalVariables|Setindex (+ (LocalVariables|Getindex) 3))))

(fn ShowThrustVertexDirection
  (for (_array_element _array_index) (Variables|Default|GetVertexDirection)
    (Transformation|SetRelativeRotation (Utilities|Array|Get(acopy) (Variables|Default|GetVertexRotateDirection) _array_index) (Math|Rotator|MakeRotfromXZ _array_element (Math|Vector|Normalize (Math|Vector|CrossProduct _array_element "0,1.000000,0.000000"))) false)))

(fn InitVertexRotateDirection
  (Utilities|Array|Resize (Variables|Default|GetVertexRotateDirection) 8)
  (Utilities|Array|SetArrayElem (Variables|Default|GetVertexRotateDirection) 0 (Variables|Default|GetArrowRotate1))
  (Utilities|Array|SetArrayElem (Variables|Default|GetVertexRotateDirection) 1 (Variables|Default|GetArrowRotate2))
  (Utilities|Array|SetArrayElem (Variables|Default|GetVertexRotateDirection) 2 (Variables|Default|GetArrowRotate3))
  (Utilities|Array|SetArrayElem (Variables|Default|GetVertexRotateDirection) 3 (Variables|Default|GetArrowRotate4))
  (Utilities|Array|SetArrayElem (Variables|Default|GetVertexRotateDirection) 4 (Variables|Default|GetArrowRotate5))
  (Utilities|Array|SetArrayElem (Variables|Default|GetVertexRotateDirection) 5 (Variables|Default|GetArrowRotate6))
  (Utilities|Array|SetArrayElem (Variables|Default|GetVertexRotateDirection) 6 (Variables|Default|GetArrowRotate7))
  (Utilities|Array|SetArrayElem (Variables|Default|GetVertexRotateDirection) 7 (Variables|Default|GetArrowRotate8)))

(fn InitTangentSpaceTransform
  (Utilities|Array|Resize (Variables|Default|GetTangentSpaceTransforms) 8)
  ;[1 1 1] Thrust Vertex1 Tangent Space
  (Utilities|Array|SetArrayElem (Variables|Default|GetTangentSpaceTransforms) 0 (Math|Transform|MakeTransform "0, 0, 0" (Math|Rotator|MakeRotfromXY (Math|Vector|GetForwardVector (Variables|/Script/Engine.SceneComponent|GetRelativeRotation (Variables|Default|GetThrush1_X))) (Math|Vector|GetForwardVector (Variables|/Script/Engine.SceneComponent|GetRelativeRotation (Variables|Default|GetThrush1_Y))))))
  ;[1 1 1] Thrust Vertex2 Tangent Space
  (Utilities|Array|SetArrayElem (Variables|Default|GetTangentSpaceTransforms) 1 (Math|Transform|MakeTransform "0, 0, 0" (Math|Rotator|MakeRotfromXY (Math|Vector|NegateVector (Math|Vector|GetForwardVector (Variables|/Script/Engine.SceneComponent|GetRelativeRotation (Variables|Default|GetThrust2_NX)))) (Math|Vector|GetForwardVector (Variables|/Script/Engine.SceneComponent|GetRelativeRotation (Variables|Default|GetThrust2_Y))))))
  ;[1 1 1] Thrust Vertex3 Tangent Space
  (Utilities|Array|SetArrayElem (Variables|Default|GetTangentSpaceTransforms) 2 (Math|Transform|MakeTransform "0, 0, 0" (Math|Rotator|MakeRotfromXY (Math|Vector|NegateVector (Math|Vector|GetForwardVector (Variables|/Script/Engine.SceneComponent|GetRelativeRotation (Variables|Default|GetThrust3_NX)))) (Math|Vector|NegateVector (Math|Vector|GetForwardVector (Variables|/Script/Engine.SceneComponent|GetRelativeRotation (Variables|Default|GetThrust3_NY)))))))
  ;[1 1 1] Thrust Vertex4 Tangent Space
  (Utilities|Array|SetArrayElem (Variables|Default|GetTangentSpaceTransforms) 3 (Math|Transform|MakeTransform "0, 0, 0" (Math|Rotator|MakeRotfromXY (Math|Vector|GetForwardVector (Variables|/Script/Engine.SceneComponent|GetRelativeRotation (Variables|Default|GetThrust4_X))) (Math|Vector|NegateVector (Math|Vector|GetForwardVector (Variables|/Script/Engine.SceneComponent|GetRelativeRotation (Variables|Default|GetThrust4_NY)))))))
  ;[1 1 1] Thrust Vertex5 Tangent Space
  (Utilities|Array|SetArrayElem (Variables|Default|GetTangentSpaceTransforms) 4 (Math|Transform|MakeTransform "0, 0, 0" (Math|Rotator|MakeRotfromXY (Math|Vector|GetForwardVector (Variables|/Script/Engine.SceneComponent|GetRelativeRotation (Variables|Default|GetThrust5_X))) (Math|Vector|GetForwardVector (Variables|/Script/Engine.SceneComponent|GetRelativeRotation (Variables|Default|GetThrust5_Y))))))
  ;[1 1 1] Thrust Vertex6 Tangent Space
  (Utilities|Array|SetArrayElem (Variables|Default|GetTangentSpaceTransforms) 5 (Math|Transform|MakeTransform "0, 0, 0" (Math|Rotator|MakeRotfromXY (Math|Vector|NegateVector (Math|Vector|GetForwardVector (Variables|/Script/Engine.SceneComponent|GetRelativeRotation (Variables|Default|GetThrust6_NX)))) (Math|Vector|GetForwardVector (Variables|/Script/Engine.SceneComponent|GetRelativeRotation (Variables|Default|GetThrust6_Y))))))
  ;[1 1 1] Thrust Vertex7 Tangent Space
  (Utilities|Array|SetArrayElem (Variables|Default|GetTangentSpaceTransforms) 6 (Math|Transform|MakeTransform "0, 0, 0" (Math|Rotator|MakeRotfromXY (Math|Vector|NegateVector (Math|Vector|GetForwardVector (Variables|/Script/Engine.SceneComponent|GetRelativeRotation (Variables|Default|GetThrust7_NX)))) (Math|Vector|NegateVector (Math|Vector|GetForwardVector (Variables|/Script/Engine.SceneComponent|GetRelativeRotation (Variables|Default|GetThrust7_NY))))) "1,1,1.000000"))
  ;[1 1 1] Thrust Vertex8 Tangent Space
  (Utilities|Array|SetArrayElem (Variables|Default|GetTangentSpaceTransforms) 7 (Math|Transform|MakeTransform "0, 0, 0" (Math|Rotator|MakeRotfromXY (Math|Vector|GetForwardVector (Variables|/Script/Engine.SceneComponent|GetRelativeRotation (Variables|Default|GetThrust8_X))) (Math|Vector|NegateVector (Math|Vector|GetForwardVector (Variables|/Script/Engine.SceneComponent|GetRelativeRotation (Variables|Default|GetThrust8_NY))))))))

(fn ThrustbyVector
  (params (ThrustVertexIndex :type Integer) (ThrustVector :type Vector) (ThrustPower0 :type Float%20%28single-precision%29))
  (LocalVariables|SetThrustPower ThrustPower0)
  (LocalVariables|SetThrustIndex (* ThrustVertexIndex 3))
  (Utilities|FlowControl|Sequence
    (:then_0
      ;[1 1 1] Thrust X
      (if (not (< (Math|Vector|DotProduct (Math|Vector|GetForwardVector (Transformation|GetWorldRotation (Utilities|Array|Get(acopy) (Variables|Default|GetThrustes) (LocalVariables|GetThrustIndex)))) ThrustVector) 0.0))
        (CallFunction|Thrust (LocalVariables|GetThrustIndex) (* (Math|Vector|DotProduct (Math|Vector|GetForwardVector (Transformation|GetWorldRotation (Utilities|Array|Get(acopy) (Variables|Default|GetThrustes) (LocalVariables|GetThrustIndex)))) ThrustVector) (LocalVariables|GetThrustPower)))))
    (:then_1
      ;[1 1 1] Thrust Y
      (LocalVariables|SetThrustIndex (+ (LocalVariables|GetThrustIndex) 1))
      (if (not (< (Math|Vector|DotProduct (Math|Vector|GetForwardVector (Transformation|GetWorldRotation (Utilities|Array|Get(acopy) (Variables|Default|GetThrustes) (LocalVariables|GetThrustIndex)))) ThrustVector) 0.0))
        (CallFunction|Thrust (LocalVariables|GetThrustIndex) (* (Math|Vector|DotProduct (Math|Vector|GetForwardVector (Transformation|GetWorldRotation (Utilities|Array|Get(acopy) (Variables|Default|GetThrustes) (LocalVariables|GetThrustIndex)))) ThrustVector) (LocalVariables|GetThrustPower)))))
    (:then_2
      ;[1 1 1] Thrust Z
      (LocalVariables|SetThrustIndex (+ (LocalVariables|GetThrustIndex) 1))
      (if (not (< (Math|Vector|DotProduct (Math|Vector|GetForwardVector (Transformation|GetWorldRotation (Utilities|Array|Get(acopy) (Variables|Default|GetThrustes) (LocalVariables|GetThrustIndex)))) ThrustVector) 0.0))
        (CallFunction|Thrust (LocalVariables|GetThrustIndex) (* (Math|Vector|DotProduct (Math|Vector|GetForwardVector (Transformation|GetWorldRotation (Utilities|Array|Get(acopy) (Variables|Default|GetThrustes) (LocalVariables|GetThrustIndex)))) ThrustVector) (LocalVariables|GetThrustPower)))))))

(fn Update
  (params (DeltaSeconds :type Float%20%28single-precision%29))
  (bind _thrustofftimer (Variables|Default|GetThrustOffTimer))
  (for (_array_element _array_index) _thrustofftimer
    (if (> _array_element 0.0)
      (Utilities|Array|SetArrayElem _thrustofftimer _array_index (- _array_element DeltaSeconds))
      (if (< (Utilities|Array|Get(acopy) _thrustofftimer _array_index) 0.0)
        (CallFunction|ThrustOff _array_index))))
  ;[1 1 1] Lift Power
  (Physics|AddImpulse (Variables|Default|GetStaticMesh1) (* "0,0.000000,1.000000" (* DeltaSeconds 9.6e+02)) "None" true)
  ;[1 1 1] Hover
  (CallFunction|Hover 5e+02))

(fn ThrustbyVector2
  (params (ThrustVertexIndex :type Integer) (ThrustVector :type Vector))
  (LocalVariables|SetThrustPower 1e+03)
  (LocalVariables|SetThrustIndex (* ThrustVertexIndex 3))
  (Utilities|FlowControl|Sequence
    (:then_0
      ;[1 1 1] Thrust X
      (if (not (< (Math|Vector|DotProduct (Math|Vector|GetForwardVector (Transformation|GetWorldRotation (Utilities|Array|Get(acopy) (Variables|Default|GetThrustes) (LocalVariables|GetThrustIndex)))) ThrustVector) 0.0))
        (CallFunction|Thrust (LocalVariables|GetThrustIndex) (* (Math|Vector|DotProduct (Math|Vector|GetForwardVector (Transformation|GetWorldRotation (Utilities|Array|Get(acopy) (Variables|Default|GetThrustes) (LocalVariables|GetThrustIndex)))) ThrustVector) (LocalVariables|GetThrustPower)))))
    (:then_1
      ;[1 1 1] Thrust Y
      (LocalVariables|SetThrustIndex (+ (LocalVariables|GetThrustIndex) 1))
      (if (not (< (Math|Vector|DotProduct (Math|Vector|GetForwardVector (Transformation|GetWorldRotation (Utilities|Array|Get(acopy) (Variables|Default|GetThrustes) (LocalVariables|GetThrustIndex)))) ThrustVector) 0.0))
        (CallFunction|Thrust (LocalVariables|GetThrustIndex) (* (Math|Vector|DotProduct (Math|Vector|GetForwardVector (Transformation|GetWorldRotation (Utilities|Array|Get(acopy) (Variables|Default|GetThrustes) (LocalVariables|GetThrustIndex)))) ThrustVector) (LocalVariables|GetThrustPower)))))
    (:then_2
      ;[1 1 1] Thrust Z
      (LocalVariables|SetThrustIndex (+ (LocalVariables|GetThrustIndex) 1))
      (if (not (< (Math|Vector|DotProduct (Math|Vector|GetForwardVector (Transformation|GetWorldRotation (Utilities|Array|Get(acopy) (Variables|Default|GetThrustes) (LocalVariables|GetThrustIndex)))) ThrustVector) 0.0))
        (CallFunction|Thrust (LocalVariables|GetThrustIndex) (* (Math|Vector|DotProduct (Math|Vector|GetForwardVector (Transformation|GetWorldRotation (Utilities|Array|Get(acopy) (Variables|Default|GetThrustes) (LocalVariables|GetThrustIndex)))) ThrustVector) (LocalVariables|GetThrustPower)))))))

(fn Move
  (params (ThrustVector :type Vector) (ThrustPower :type Float%20%28single-precision%29))
  (for (_ _array_index) (Variables|Default|GetThrustes)
    (CallFunction|ThrustbyVector _array_index ThrustVector ThrustPower)))

(fn Hover
  (params (Stay%20Height :type Float%20%28single-precision%29))
  (if (< (.Z (Math|Vector|BreakVector (Transformation|GetWorldLocation (Variables|Default|GetStaticMesh1)))) Stay%20Height)
    (CallFunction|Move "0, 0,1.000000" 1e+03)))